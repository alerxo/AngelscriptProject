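; BP_FireBall is a fireball ability actor that deals an area gameplay effect on impact using the Gameplay Ability System.
; Its sphere starts at zero scale and lerps toward a target scale each tick.
; On hit, it applies its spec handle from the owner's ability system to overlapped actors with ability systems within a radius.
; It then spawns a Niagara impact effect and destroys itself.
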(event `self.ReceiveBeginPlay`
  (`SceneComponent.SetRelativeScale3D` (`self.Sphere`) (0.0 0.0 0.0)))

(event `self.ReceiveTick`
  (params (DeltaSeconds :type "Float (single-precision)"))
  (bind _sphere (`self.Sphere`))
  (`SceneComponent.SetRelativeScale3D` _sphere (`KismetMathLibrary.VLerp` (`SceneComponent.K2_GetComponentScale` _sphere) (`self.Scale`) (* (`self.ScaleSpeed`) DeltaSeconds))))

(event `self.ReceiveHit`
  (params (MyComp :type "PrimitiveComponent Object Reference") (Other :type "Actor Object Reference") (OtherComp :type "PrimitiveComponent Object Reference") (bSelfMoved :type Boolean) (HitLocation :type "Vector Structure") (HitNormal :type "Vector Structure") (NormalImpulse :type "Vector Structure") (Hit :type "HitResult Structure (by ref)"))
  (bind _returnvalue (`AbilitySystemBlueprintLibrary.GetAbilitySystemComponent` (`self.GetOwner`)))
  (`/Engine/EditorBlueprintResources/StandardMacros.IsValid` _returnvalue
    (:`Is Valid`
      ; Overlap actors and apply spec handle
      (bind _outactors (`KismetSystemLibrary.SphereOverlapActors` HitLocation (`self.Radius`) (`self.Object Types`)))
      (for _array_element _outactors
        (bind _returnvalue_2 (`AbilitySystemBlueprintLibrary.GetAbilitySystemComponent` _array_element))
        (`/Engine/EditorBlueprintResources/StandardMacros.IsValid` _returnvalue_2
          (:`Is Valid`
            (`AbilitySystemComponent.BP_ApplyGameplayEffectSpecToTarget` _returnvalue (`self.SpecHandle`) _returnvalue_2)))))
    (:`Is Not Valid`
      _))
  (`NiagaraFunctionLibrary.SpawnSystemAtLocation` "/Game/Ability/NS_FireBallImpact.NS_FireBallImpact" HitLocation)
  (`self.K2_DestroyActor`))

(fn `UserConstructionScript`)