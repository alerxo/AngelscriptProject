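; Gameplay ability that casts a fireball: plays a sword-and-shield casting montage and reacts to its gameplay event tags.
; On cast start it spawns BP_FireBall_Angel ahead of the left hand, gives it a GE_Damage spec with SetByCaller damage, and attaches it to that hand.
; On cast end it detaches and launches the fireball along the owner's forward vector with set gravity, then ends.
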(event `self.K2_ActivateAbility`
  (bind _returnvalue (`self.GetOwningActorFromActorInfo`))
  (bind _returnvalue_location (`KismetMathLibrary.BreakTransform` (`SkinnedMeshComponent.GetBoneTransform` (`self.GetOwningComponentFromActorInfo`) "hand_l" "RTS_World")))
  (`AbilityTask_PlayMontageAndWait.CreatePlayMontageAndWaitProxy` "None" "/Game/Characters/Mannequins/Anims/SwordShield/Sword_And_Shield_Casting_Montage.Sword_And_Shield_Casting_Montage"
    (:`then`
      (bind (_asynctaskproxy _payload) (`AbilityTask_WaitGameplayEvent.WaitGameplayEvent` (struct :`TagName` "Event.Anim.Cast") null false false)
        (:`EventReceived`
          (`|SwitchGameplayTag` (break `GameplayEventData` _payload)
            (:`Event.Anim.Cast.Start`
              (bind _aspawn (cast `Pawn` _returnvalue))
              (bind _returnvalue_2 (`|SpawnActorFromClass` "/Game/Ability/BP_FireBall_Angel.BP_FireBall_Angel_C" (`KismetMathLibrary.MakeTransform` (+ _returnvalue_location (* (`self.SpawnDistance`) (`SceneComponent.GetForwardVector` (`Actor.RootComponent` _returnvalue))))) "Undefined" "MultiplyWithRoot" null _aspawn))
              ; Initialize fireball
              (bind _returnvalue_3 (`AbilitySystemBlueprintLibrary.AssignTagSetByCallerMagnitude` (`self.MakeOutgoingGameplayEffectSpec` "/Game/Ability/GE_Damage.GE_Damage_C") (struct :`TagName` "SetByCaller.DamageAmount") (`self.Damage`)))
              (`FireBall_Angel.SetHandle` _returnvalue_2 _returnvalue_3)
              (`Actor.SetOwner` _returnvalue_2 (`self.GetOwningActorFromActorInfo`))
              (`Actor.K2_AttachToComponent` _returnvalue_2 (`self.GetOwningComponentFromActorInfo`) "hand_l" "KeepWorld" "KeepRelative" "KeepRelative" true))
            (:`Event.Anim.Cast.End`
              ; Detach and launch fireball
              (if (`KismetSystemLibrary.IsValid` _returnvalue_2)
                (`SceneComponent.K2_DetachFromComponent` (`Actor.RootComponent` _returnvalue_2) "KeepWorld" "KeepRelative" "KeepRelative" true)
                (bind _projectilemovement (`/Game/Ability/BP_FireBall_Angel.ProjectileMovement` _returnvalue_2))
                (set `MovementComponent.Velocity` (* (`self.Velocity`) (`Actor.GetActorForwardVector` (`self.GetOwningActorFromActorInfo`))) _projectilemovement)
                (set `ProjectileMovementComponent.ProjectileGravityScale` (`self.Gravity`) _projectilemovement)
                (`self.K2_EndAbility`)
                (else
                  (`self.K2_EndAbility`))))))))
    (:`OnCompleted`
      (`self.K2_EndAbility` :!label _label))
    (:`OnInterrupted`
      (goto _label))
    (:`OnCancelled`
      (goto _label))))