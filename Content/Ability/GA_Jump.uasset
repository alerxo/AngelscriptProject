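; Gameplay Ability that makes the owning Character jump.
; On activation it calls Jump, then polls the root component's vertical velocity through a short looping Delay until the character stops rising.
; It then ends itself, at the apex rather than on landing, and OnEndAbility calls StopJumping on the Character.
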(event `self.K2_ActivateAbility`
  (bind (_returnvalue_x _returnvalue_y _returnvalue_z) (`KismetMathLibrary.BreakVector` (`SceneComponent.GetComponentVelocity` (`Actor.RootComponent` (`self.GetOwningActorFromActorInfo`)))))
  (bind _ascharacter (cast `Character` (`self.GetOwningActorFromActorInfo`)))
  (`Character.Jump` _ascharacter)
  (`KismetSystemLibrary.Delay` 0.1 :!label _label)
  (if (> _returnvalue_z 0.0)
    (goto _label)
    (else
      (`self.K2_EndAbility`))))

(event `self.K2_OnEndAbility`
  (params (bWasCancelled :type Boolean))
  (bind _ascharacter (cast `Character` (`self.GetOwningActorFromActorInfo`)))
  (`Character.StopJumping` _ascharacter))