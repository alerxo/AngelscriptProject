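; Target dummy character that reacts to health changes with montages and a white flash, and respawns after death.
; NotifyHealthAttributeChanged ignores changes from zero, plays an impact montage for any nonzero result, and on zero disables capsule collision and plays a death montage.
; The flash briefly swaps both mesh materials to M_Damaged.
; After the death montage and an extra delay, it spawns a fresh dummy at its transform and destroys itself.
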(event `self.NotifyHealthAttributeChanged`
  (params (OldValue :type "Float (single-precision)") (NewValue :type "Float (single-precision)"))
  ; Check health
  (if (== OldValue 0.0)
    _
    (elif (== NewValue 0.0)
      (`PrimitiveComponent.SetCollisionEnabled` (`self.CapsuleComponent`) "NoCollision")
      (bind _returnvalue (`self.PlayAnimMontage` "/Game/Characters/Mannequins/Anims/SwordShield/Falling_Back_Death_Montage.Falling_Back_Death_Montage"))
      ; Flash White
      (`self.SetMaterialWhite`)
      (`KismetSystemLibrary.Delay` (`self.FlashDuration`))
      (`self.SetMaterialDefault`)
      (`KismetSystemLibrary.Delay` (+ _returnvalue (`self.DeathDuration`)))
      ; Spawn new TargetDummy
      (`|SpawnActorFromClass` "BP_TargetDummy_C" (`self.GetTransform` self) "Undefined" "MultiplyWithRoot" null null)
      (`self.K2_DestroyActor`)
      (else
        (`self.PlayAnimMontage` "/Game/Characters/Mannequins/Anims/SwordShield/Sword_And_Shield_Impact_Montage.Sword_And_Shield_Impact_Montage")
        ; Flash White
        (`self.SetMaterialWhite`)
        (`KismetSystemLibrary.Delay` (`self.FlashDuration`))
        (`self.SetMaterialDefault`)))))

(fn `SetMaterialDefault`
  (bind _mesh (`self.Mesh`))
  (`PrimitiveComponent.SetMaterial` _mesh 0 "/Game/Characters/Mannequins/Materials/Manny/MI_Manny_01_New.MI_Manny_01_New")
  (`PrimitiveComponent.SetMaterial` _mesh 1 "/Game/Characters/Mannequins/Materials/Manny/MI_Manny_02_New.MI_Manny_02_New"))

(fn `SetMaterialWhite`
  (bind _mesh (`self.Mesh`))
  (`PrimitiveComponent.SetMaterial` _mesh 0 "/Game/Characters/Mannequins/Materials/Manny/M_Damaged.M_Damaged")
  (`PrimitiveComponent.SetMaterial` _mesh 1 "/Game/Characters/Mannequins/Materials/Manny/M_Damaged.M_Damaged"))

(fn `UserConstructionScript`
  (`parent.UserConstructionScript`))